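; BP_DummyTarget is a pawn Blueprint whose only logic is pause menu handling.
; The Pause input action calls PauseGame, which pauses the game, lazily creates and caches a BP_Pause widget, then shows it with UI-only input and a visible cursor.
; UnPause reverses this by resuming the game, removing the widget, restoring game-only input and hiding the cursor, though nothing in this Blueprint calls it.
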(event EventBeginPlay)

(event Collision|EventActorBeginOverlap
  (params (OtherActor :type Actor%20Object%20Reference)))

(event EventTick
  (params (DeltaSeconds :type Float%20%28single-precision%29)))

(event Input|ActionEvents|InputActionPause
  (params (Key :type Key%20Structure :default "None"))
  (:Pressed
    (CallFunction|PauseGame)))

(fn ConstructionScript)

(fn PauseGame
  (bind _returnvalue (Game|GetPlayerController 0))
  (Game|SetGamePaused true)
  (Utilities|IsValid (Variables|Default|GetPauseMenu)
    (:Is%20Valid
      _)
    (:Is%20Not%20Valid
      (bind _returnvalue_2 (UserInterface|CreateWidget "/Game/Blueprints/UI/BP_Pause.BP_Pause_C" (Game|GetPlayerController 0)))
      (Variables|Default|SetPauseMenu _returnvalue_2)))
  (UserInterface|Viewport|AddtoViewport (Variables|Default|GetPauseMenu) 0)
  (Input|SetInputModeUIOnly _returnvalue (Variables|Default|GetPauseMenu) "DoNotLock")
  (Variables|/Script/Engine.PlayerController|SetbShowMouseCursor _returnvalue true))

(fn UnPause
  (bind _returnvalue (Game|GetPlayerController 0))
  (Game|SetGamePaused false)
  (Widget|RemovefromParent (Variables|Default|GetPauseMenu))
  (Input|SetInputModeGameOnly _returnvalue)
  (Variables|/Script/Engine.PlayerController|SetbShowMouseCursor _returnvalue false))